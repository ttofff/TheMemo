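; Player character for an elderly-care app that creates the main UI and runs reminders, safety monitoring and a voice assistant.
; Tick polls time against medical, pill, outdoor and indoor lists from UI, and re-samples GPS for safe-radius checks.
; Falls, leaving the radius and unconfirmed pills trigger SMS alerts.
; Mic loudness starts Azure speech recognition; Azure TTS speaks alerts, Amap weather (rain text hardcoded) and Baidu AI replies.
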(event OnAudioEnvelopeValue(AudioCapture)
  (params (EnvelopeValue :type Float%20%28single-precision%29))
  ;[1 1 1] 检测说话声
  (if (> EnvelopeValue (Variables|语音输入|GetVoice_Size))
    (Utilities|FlowControl|DoOnce false
      (:Completed
        (CallFunction|Azure(ARS))))))

(event Custom|Azure%28ATTS%29
  (params (SynthesisText :type String))
  ;[1 1 1] 语音合成
  (bind _generatedsound (|TexttoSoundWaveCustomOptions (Utilities|Struct|MakeAzSpeechSubscriptionOptions (Variables|Default|GetAzure%20API%20Key) "southeastasia" false "https://None.api.cognitive.microsoft.com/sts/v1.0/issuetoken") (Utilities|Struct|MakeAzSpeechSynthesisOptions (Variables|语音输入|GetInput_Locale) (Variables|语音输出|GetOutput_Locale)) SynthesisText)
    (:SynthesisCompleted
      (Audio|PlaySound2D _generatedsound 1.0 1.0 0.0 0 0)
      (Utilities|FlowControl|Delay 0.2))))

(event Custom|SpeechOpen
  ;[1 1 1] 开始检测语音识别
  (Utilities|IsValid (Variables|Default|GetAudioCapture)
    (:Is%20Valid
      (Variables|语音输入|SetAudio%20Input%20Text "")
      (Variables|语音输入|SetVoice_Size 0.005)
      (Default|InVoiceTip (Variables|UMG|GetAllUMG)))))

(event Custom|Get_Current_City
  (params (Request :type Va%20Rest%20Request%20JSON%20Object%20Reference))
  ;[1 1 1] 获取目前所在的城市编码
  (Variables|Weather|SetWeather_City (Class|VaRestJsonObject|GetStringField (Class|VaRestRequestJSON|GetResponseObject Request) "adcode"))
  (CallFunction|WeatherMessage))

(event Custom|CheckTimeOver
  (bind _returnvalue (Math|DateTime|Now))
  (bind (_returnvalue_2 _returnvalue2 _returnvalue3 _returnvalue4) (Utilities|CheckNumber (.month _returnvalue) (.month _returnvalue) (.day _returnvalue) (.day _returnvalue) (.hour _returnvalue) (.hour _returnvalue) (.minute _returnvalue) (.minute _returnvalue)))
  ;[1 1 1] 获取时间和数组
  (if (not (Variables|Default|GetIsBreak))
    (Utilities|IsValid (Variables|UMG|GetAllUMG)
      (:Is%20Valid
        (CallFunction|GetNotifyMessage)
        (Variables|Default|SetNowData_andTime (Utilities|String|Append (Utilities|String|ToString(Integer) (.year _returnvalue)) "年" _returnvalue_2 "月" _returnvalue2 "日" _returnvalue3 "时" _returnvalue4 "分"))
        (Variables|Default|SetNowTime (Utilities|String|Append _returnvalue3 "时" _returnvalue4 "分"))
        ;;[1 1 1] 获取周几
        (bind _returnvalue_3 (Class|TheMemoCharacter|GetDayOfWeek))
        (Variables|Default|SetNowWeekday _returnvalue_3)
        ;;[1 1 1] 实时检测信息
        (CallFunction|CheckNotify)))))

(event Custom|Reset
  ;[1 1 1] 事件Tick
  (Utilities|FlowControl|DoOnce false) ; enters at Reset
)

(event Custom|Baidu%28AI%29
  (params (Question :type String))
  (bind _currentwidget (Variables|UMG|GetCurrentWidget))
  ;[1 1 1] 智能AI
  (bind _returnvalue (Class|VaRestSubsystem|ConstructVaRestRequestExt (|VaRestSubsystem) "POST" "json"))
  (Class|VaRestRequestJSON|SetRequestObject _returnvalue (|MakeJson (Utilities|Array|MakeArray (|MakeJson "user" Question))))
  (Class|VaRestRequestJSON|SetHeader _returnvalue "Content-Type" "application/json")
  (bind _result (Class|VaRestRequestJSON|ApplyURL _returnvalue (Utilities|String|Append "https://aip.baidubce.com/oauth/2.0/token?grant_type=client_credentials&client_id=" (Variables|GBT|GetAPI%20Key) "&client_secret=" (Variables|GBT|GetSecret%20Key))))
  (bind _result_2 (Class|VaRestRequestJSON|ApplyURL _returnvalue (Utilities|String|Append "https://aip.baidubce.com/rpc/2.0/ai_custom/v1/wenxinworkshop/chat/completions?access_token=" (Class|VaRestJsonObject|GetStringField _result "access_token"))))
  (Variables|GBT|SetResponse%20Text (Class|VaRestJsonObject|GetStringField _result_2 "result"))
  (Utilities|IsValid _currentwidget
    (:Is%20Valid
      (Class|InputInterface|GetOutputText(Message) _currentwidget (Variables|GBT|GetResponse%20Text)))
    (:Is%20Not%20Valid
      _))
  (if (Variables|Default|Get%20IsNeedTalk)
    (CallFunction|Azure(ATTS) (Variables|GBT|GetResponse%20Text))))

(event Custom|AddPillTime
  (params (NotConfirmNumber :type Integer))
  (bind _returnvalue (Math|DateTime|Now))
  (bind _pill_a (Variables|UMG|GetPILL%20A))
  (bind _output (Utilities|Array|Get(acopy) _pill_a NotConfirmNumber))
  ;[1 1 1] 延长吃药时间
  (Utilities|IsValid _output
    (:Is%20Valid
      (Variables|Default|SetHour (.hour _returnvalue))
      (bind _output_get (Variables|Default|SetMinute (.minute _returnvalue)))
      (if (> (+ _output_get (Variables|Default|GetDelayPillTime)) 60)
        (Math|Integer|IncrementInt (Variables|Default|GetHour)
          (:%20%20
            (Variables|Default|SetMinute (- (+ _output_get (Variables|Default|GetDelayPillTime)) (Variables|Default|GetMinute)))))
        (else
          (Variables|Default|SetMinute (+ _output_get (Variables|Default|GetDelayPillTime)))))
      (if (>= (Variables|Default|GetHour) 24)
        (Variables|Default|SetHour 0))
      (Variables|/Game/UMG/Pill_Ui/Pill_Message_slot.Pill_Message_slot_C|SetTime _output (Utilities|String|Append (Utilities|String|Append (select (< (Variables|Default|GetHour) 10) "0" "") (Utilities|String|ToString(Integer) (Variables|Default|GetHour))) "时" (Utilities|String|Append (select (< (Variables|Default|GetMinute) 10) "0" "") (Utilities|String|ToString(Integer) (Variables|Default|GetMinute))) "分")))))

(event Custom|Send%20PhoneMessage
  (params (TemplateCode :type String))
  ;[1 1 1] 发送短信
  (bind _returnvalue (Class|InitePost|IniteConfig "LTAI5tJExn83iZNqW6yNTGcx" "6shROERDAr4YFRot1pA8NQwrVjsJ10" "乐耆岁月" TemplateCode))
  (if _returnvalue
    (|SendActivationCode "" (Variables|Default|GetPhone%20Num))))

(event Custom|LocationReset
  ;[1 1 1] 每十秒测一次位置
  (Utilities|FlowControl|DoOnce false) ; enters at Reset
)

(event Custom|WeatherMessage
  ;[1 1 1] 获取实时天气信息
  (Class|VaRestSubsystem|CallURL (|VaRestSubsystem) (Utilities|String|Append "https://restapi.amap.com/v3/weather/weatherInfo?" "city=" (Variables|Weather|GetWeather_City) "&key=" (Variables|Weather|GetWeather_API_Key)) "GET" "x_www_form_urlencoded_url" 0 (delegate Custom|Weather_Messages)))

(event Custom|Get%20Lat_Lng_Distance
  (bind _raw_lat (Variables|Default|GetRaw_lat))
  (bind _raw_lng (Variables|Default|GetRaw_lng))
  ;[1 1 1] 获取经纬度
  ;;[1 1 1] 检测距离
  (bind _returnvalue (Class|TheMemoCharacter|GetDistance (Utilities|Array|Get(acopy) (Variables|Default|GetRaw_lat)) (Utilities|Array|Get(acopy) (Variables|Default|GetRaw_lng)) (Utilities|Array|Get(acopy) _raw_lat (- (Utilities|Array|Length _raw_lat) 1)) (Utilities|Array|Get(acopy) _raw_lng (- (Utilities|Array|Length _raw_lng) 1))))
  (CallFunction|CheckOutOfRadius _returnvalue))

(event Custom|Check%20Out%20of%20Radius
  (params (Disatance :type Float%20%28double-precision%29))
  (bind _distances (Variables|Default|GetDistances))
  (bind _allumg (Variables|UMG|GetAllUMG))
  (bind _protect_ui (Variables|/Game/UMG/All_Ui.All_Ui_C|Getprotect_Ui _allumg))
  ;[1 1 1] 获取经纬度
  ;;[1 1 1] 检测是否在安全范围内
  (if (== (Utilities|Array|FindItem _distances Disatance) -1)
    (Utilities|Array|Add _distances Disatance))
  (Utilities|IsValid _allumg
    (:Is%20Valid
      (if (> (Utilities|Array|Get(acopy) _distances (- (Utilities|Array|Length _distances) 1)) (Variables|Default|GetProtectRadius))
        (Default|ProtectFaild _protect_ui)
        (Utilities|FlowControl|DoOnce false
          (:Completed
            (CallFunction|Azure(ATTS) "您已走出安全范围，请注意安全")
            (CallFunction|SendPhoneMessage "SMS_471380476")))
        (else
          (Default|ProtectSuccess _protect_ui))))))

(event Custom|SpeechStop
  ;[1 1 1] 结束检测语音识别
  (Utilities|IsValid (Variables|Default|GetAudioCapture)
    (:Is%20Valid
      (Variables|语音输入|SetVoice_Size 1e+03)
      (Default|OutVoiceTip (Variables|UMG|GetAllUMG)))))

(event Custom|CheckNotify
  ;[1 1 1] 医疗通知
  (for _array_element (Variables|UMG|GetDoctor%20A)
    (if (Utilities|String|Contains (Utilities|String|ToString(Text) (Variables|/Game/UMG/Doctor_Ui/Doctor_MEssage_Slot.Doctor_MEssage_Slot_C|Getdata_text _array_element)) (Variables|Default|GetNowData_andTime))
      (Variables|Default|SetIsYiLiao true)
      (CallFunction|Azure(ATTS) (Utilities|String|Append "现在是" (Variables|Default|GetNowTime) "，该去" (Utilities|String|ToString(Text) (Variables|/Game/UMG/Doctor_Ui/Doctor_MEssage_Slot.Doctor_MEssage_Slot_C|GetPlace_text _array_element)) "，" (Utilities|String|ToString(Text) (Variables|/Game/UMG/Doctor_Ui/Doctor_MEssage_Slot.Doctor_MEssage_Slot_C|GetDoctor_text _array_element)) "了。"))
      (Default|ToNotifyAnimation (Variables|UMG|GetAllUMG) "医疗预约提醒" (Utilities|Text|ToText(String) (Utilities|String|Append "现在是" (Variables|Default|GetNowTime) "，该去" (Utilities|String|ToString(Text) (Variables|/Game/UMG/Doctor_Ui/Doctor_MEssage_Slot.Doctor_MEssage_Slot_C|GetPlace_text _array_element)) "，" (Utilities|String|ToString(Text) (Variables|/Game/UMG/Doctor_Ui/Doctor_MEssage_Slot.Doctor_MEssage_Slot_C|GetDoctor_text _array_element)) "了。")))
      (Variables|Default|SetIsBreak true)))
  ;[1 1 1] 用药通知
  (for (_array_element_2 _array_index) (Variables|UMG|GetPILL%20A)
    (if (Utilities|String|Contains (Variables|/Game/UMG/Pill_Ui/Pill_Message_slot.Pill_Message_slot_C|GetTime _array_element_2) (Variables|Default|GetNowTime))
      (CallFunction|Azure(ATTS) (Utilities|String|Append "该服用" (Utilities|String|ToString(Text) (Variables|/Game/UMG/Pill_Ui/Pill_Message_slot.Pill_Message_slot_C|Getmessage_text _array_element_2)) "了。"))
      (Default|ToNotifyAnimation (Variables|UMG|GetAllUMG) "用药提醒" (Utilities|Text|ToText(String) (Utilities|String|Append "该服用" (Utilities|String|ToString(Text) (Variables|/Game/UMG/Pill_Ui/Pill_Message_slot.Pill_Message_slot_C|Getmessage_text _array_element_2)) "了。")) _array_index)
      (Variables|Default|SetIsBreak true)
      (if (>= (Variables|Default|GetNotConfirmPill_Number) 2)
        (CallFunction|SendPhoneMessage "SMS_469080788")
        (Variables|Default|SetNotConfirmPill_Number 0))))
  ;[1 1 1] 户外通知
  (for _array_element_3 (Variables|UMG|GetOUTSIDE%20A)
    (if (and (Utilities|String|Contains (Utilities|String|ToString(Text) (Variables|/Game/UMG/Outside_Ui/Outside_Message_slot.Outside_Message_slot_C|Gettime_text _array_element_3)) (Variables|Default|GetNowTime)) (Utilities|String|Contains (Utilities|String|ToString(Text) (Variables|/Game/UMG/Outside_Ui/Outside_Message_slot.Outside_Message_slot_C|Getdata_text _array_element_3)) (Variables|Default|GetNowWeekday)))
      (CallFunction|Azure(ATTS) (Utilities|String|Append "现在是" (Variables|Default|GetNowTime) "，该" (Utilities|String|ToString(Text) (Variables|/Game/UMG/Outside_Ui/Outside_Message_slot.Outside_Message_slot_C|Getmessage_text _array_element_3)) "了。"))
      (Default|ToNotifyAnimation (Variables|UMG|GetAllUMG) "户外提醒" (Utilities|Text|ToText(String) (Utilities|String|Append "现在是" (Variables|Default|GetNowTime) "，该" (Utilities|String|ToString(Text) (Variables|/Game/UMG/Outside_Ui/Outside_Message_slot.Outside_Message_slot_C|Getmessage_text _array_element_3)) "了。")))
      (Variables|Default|SetIsBreak true)
      (Utilities|FlowControl|Delay 3.0)
      (CallFunction|GetCurrentWeather)))
  ;[1 1 1] 室内通知
  (for _array_element_4 (Variables|UMG|GetINSIDE%20A)
    (if (and (Utilities|String|Contains (Utilities|String|ToString(Text) (Variables|/Game/UMG/Inside_Ui/Inside_Message_slot.Inside_Message_slot_C|Gettime_text _array_element_4)) (Variables|Default|GetNowTime)) (Utilities|String|Contains (Utilities|String|ToString(Text) (Variables|/Game/UMG/Inside_Ui/Inside_Message_slot.Inside_Message_slot_C|Getdata_text _array_element_4)) (Variables|Default|GetNowWeekday)))
      (Default|ToNotifyAnimation (Variables|UMG|GetAllUMG) "室内提醒" (Utilities|Text|ToText(String) (Utilities|String|Append "现在是" (Variables|Default|GetNowTime) "，该" (Utilities|String|ToString(Text) (Variables|/Game/UMG/Inside_Ui/Inside_Message_slot.Inside_Message_slot_C|Getmessage_text _array_element_4)) "了。")))
      (Variables|Default|SetIsBreak true)
      (CallFunction|Azure(ATTS) (Utilities|String|Append "现在是" (Variables|Default|GetNowTime) "，该" (Utilities|String|ToString(Text) (Variables|/Game/UMG/Inside_Ui/Inside_Message_slot.Inside_Message_slot_C|Getmessage_text _array_element_4)) "了。"))))
  (CallFunction|Reset))

(event Custom|OnLocationChanged
  (params (LocationData :type Location%20Services%20Data%20Structure))
  (bind _raw_lng (Variables|Default|GetRaw_lng))
  ;[1 1 1] 获取经纬度
  (if (== (Utilities|Array|FindItem _raw_lng (.longitude LocationData)) -1)
    (Utilities|Array|Add _raw_lng (.longitude LocationData)))
  (if (== (Utilities|Array|FindItem (Variables|Default|GetRaw_lat) (.latitude LocationData)) -1)
    (Utilities|Array|Add (Variables|Default|GetRaw_lat) (.latitude LocationData))
    (CallFunction|GetLatLngDistance)))

(event Custom|Azure%28ARS%29
  ;[1 1 1] 语音识别
  (bind _finalstring (|SpeechtoTextCustomOptions (Utilities|Struct|MakeAzSpeechSubscriptionOptions (Variables|Default|GetAzure%20API%20Key) "southeastasia" false "https://None.api.cognitive.microsoft.com/sts/v1.0/issuetoken") (Utilities|Struct|MakeAzSpeechRecognitionOptions (Variables|语音输入|GetInput_Locale) false) "Default" "None")
    (:RecognitionCompleted
      _)
    (:RecognitionFailed
      _))
  (CallFunction|Rest)
  (bind _output_get (Variables|语音输入|SetAudio%20Input%20Text _finalstring))
  (if (> (Utilities|String|Len _output_get) 0)
    (if (Variables|Default|GetIsFindVoice)
      (Default|OpenUIbyVoice (Variables|UMG|GetAllUMG) (Variables|语音输入|GetAudio%20Input%20Text))
      (Variables|Default|SetIsFindVoice false)
      (else
        (Class|InputInterface|GetInputText(Message) (Variables|UMG|GetCurrentWidget) (Variables|语音输入|GetAudio%20Input%20Text))))))

(event Custom|Rest
  ;[1 1 1] 检测说话声
  (Utilities|FlowControl|DoOnce false) ; enters at Reset
)

(event Custom|Get_Current_Weather
  ;[1 1 1] 获取目前所在的城市编码
  (Class|VaRestSubsystem|CallURL (|VaRestSubsystem) (Utilities|String|Append "https://restapi.amap.com/v3/ip?" "&key=" (Variables|Weather|GetWeather_API_Key)) "GET" "x_www_form_urlencoded_url" 0 (delegate Custom|Get_Current_City)))

(event Custom|GetLocationServices
  ;[1 1 1] 获取经纬度
  (Class|LocationServices|InitLocationServices "LA_TenMeters" 1e+03 1e-06)
  (bind _returnvalue (Class|LocationServices|StartLocationServices))
  (if _returnvalue
    (bind _returnvalue_2 (Class|LocationServices|GetLocationServicesImpl))
    (EventDispatchers|BindEventtoOnLocationChanged _returnvalue_2 (delegate Custom|OnLocationChanged))))

(event Custom|ReportWeather
  ;[1 1 1] 播报天气情况
  (Variables|Default|Set%20IsNeedTalk true)
  (CallFunction|Baidu(AI) (Variables|Weather|GetWeather_Questions))
  (Default|WeatherAppear (Variables|/Game/UMG/All_Ui.All_Ui_C|GetOutside_Ui (Variables|UMG|GetAllUMG))))

(event Custom|Weather_Messages
  (params (Request :type Va%20Rest%20Request%20JSON%20Object%20Reference))
  (bind _returnvalue (Class|VaRestRequestJSON|GetResponseObject Request))
  (bind _allumg (Variables|UMG|GetAllUMG))
  (bind _returnvalue_2 (Class|VaRestJsonObject|GetObjectArrayField _returnvalue "lives"))
  (bind _outside_ui (Variables|/Game/UMG/All_Ui.All_Ui_C|GetOutside_Ui _allumg))
  (bind _output (Utilities|Array|Get(acopy) _returnvalue_2))
  (bind _returnvalue_3 (Class|VaRestJsonObject|GetStringField _output "temperature_float"))
  (bind _returnvalue_4 (Class|VaRestJsonObject|GetStringField _output "humidity_float"))
  ;[1 1 1] 获取实时天气信息
  (Variables|Weather|SetWeather_Questions (Utilities|String|Append (Variables|Weather|GetA) "大雨" (Variables|Weather|GetC) _returnvalue_3 (Variables|Weather|GetE) _returnvalue_4 (Variables|Weather|GetG)))
  (Variables|/Game/UMG/Outside_Ui/Outside_Ui.Outside_Ui_C|Setsheshidu _outside_ui (Utilities|Text|ToText(String) _returnvalue_3))
  (Variables|/Game/UMG/Outside_Ui/Outside_Ui.Outside_Ui_C|Setshidu _outside_ui (Utilities|Text|ToText(String) _returnvalue_4))
  (Utilities|FlowControl|Delay 3.0)
  (CallFunction|Azure(ATTS) (Utilities|String|Append (Variables|Weather|GetA) "大雨" (Variables|Weather|GetC) _returnvalue_3 (Variables|Weather|GetE) _returnvalue_4))
  (Utilities|FlowControl|Delay 3.5)
  (CallFunction|ReportWeather))

(event EventBeginPlay
  ;[1 1 1] 主界面初始化
  (bind _returnvalue (UserInterface|CreateWidget "/Game/UMG/All_Ui.All_Ui_C"))
  (UserInterface|Viewport|AddtoViewport _returnvalue 0)
  (Variables|UMG|SetAllUMG _returnvalue))

(event EventGetCurrentWidget
  (params (CurrentWidget :type User%20Widget%20Object%20Reference))
  ;[1 1 1] 获取当前所在的用户控件
  (Variables|UMG|SetCurrentWidget CurrentWidget))

(event EventTick
  (params (DeltaSeconds :type Float%20%28single-precision%29))
  ;[1 1 1] 事件Tick
  (Utilities|FlowControl|Sequence
    (:then_0
      (Utilities|FlowControl|DoOnce false
        (:Completed
          (CallFunction|CheckTimeOver))))
    (:then_1
      ;[1 1 1] 每十秒测一次位置
      (if (Variables|Default|GetIsInitLngAndLat)
        (Utilities|FlowControl|DoOnce false
          (:Completed
            (CallFunction|GetLocationServices)
            (Utilities|FlowControl|Delay 5.0)
            (CallFunction|LocationReset)))))))

(event Input|KeyboardEvents|RotationRate
  (params (AxisValue :type Vector :default "0, 0, 0"))
  ;[1 1 1] 跌倒检测
  (bind _length (CallFunction|FellDown AxisValue))
  (if (> _length 2e+01)
    (Utilities|FlowControl|DoOnce false
      (:Completed
        (CallFunction|SendPhoneMessage "SMS_472095005")))))

(fn ConstructionScript)

(fn GetNotifyMessage
  (bind _allumg (Variables|UMG|GetAllUMG))
  (bind _allumg_2 (Variables|UMG|GetAllUMG))
  (Variables|UMG|SetDoctor%20A (Variables|/Game/UMG/Doctor_Ui/Doctor_Ui.Doctor_Ui_C|GetDoctor_A (Variables|/Game/UMG/All_Ui.All_Ui_C|GetDoctor_Ui _allumg)))
  (Variables|UMG|SetINSIDE%20A (Variables|/Game/UMG/Inside_Ui/Inside_Ui.Inside_Ui_C|GetINSIDE_A (Variables|/Game/UMG/All_Ui.All_Ui_C|GetInside_Ui _allumg)))
  (Variables|UMG|SetOUTSIDE%20A (Variables|/Game/UMG/Outside_Ui/Outside_Ui.Outside_Ui_C|GetOUTSIDE_A (Variables|/Game/UMG/All_Ui.All_Ui_C|GetOutside_Ui _allumg_2)))
  (Variables|UMG|SetPILL%20A (Variables|/Game/UMG/Pill_Ui/Pill_Ui.Pill_Ui_C|GetPILL_A (Variables|/Game/UMG/All_Ui.All_Ui_C|GetPill_Ui _allumg_2))))

(fn FellDown
  (params (RotationRate :type Vector))
  (bind (_x _y _z) (Math|Vector|BreakVector RotationRate))
  (return (Math|Float|Sqrt (+ (Math|Float|Power _x 2.0) (Math|Float|Power _y 2.0) (Math|Float|Power _z 2.0)))))